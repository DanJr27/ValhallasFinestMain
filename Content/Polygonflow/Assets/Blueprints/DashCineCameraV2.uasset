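; DashCineCameraV2 is a cine camera Blueprint that exposes look and lens controls as its own variables.
; ComputeProperties, run on construction and every Tick, rebuilds the camera's post-process settings for grading, exposure, bloom and film effects.
; It creates fresh dynamic material instances each call for pre-tonemap outlines and post-tonemap distortion and color correction.
; Unless ControlCameraFromUEDetailsPanel is set, it also overwrites focus, filmback, lens, focal length and aperture.
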(event Custom|ComputeProperties
  (bind _returnvalue (Math|Float|MakeLiteralFloat 1.0))
  (bind _film_grain_scale (Variables|DashPostProcess/MaterialProperties|GetFilm%20Grain%20Scale))
  ;[1 0.8918 0.2289] Outline
  (bind _asmaterial (Utilities|Casting|CastToMaterial (Variables|DashPostProcess/MaterialProperties|GetPre%20ToneMapping)))
  (bind _returnvalue_2 (Rendering|Material|CreateDynamicMaterialInstance _asmaterial "None" "None" :!class /Script/Engine.KismetMaterialLibrary))
  (Rendering|Material|SetScalarParameterValue _returnvalue_2 "Outline Intensity" (Variables|DashExtras|GetOutline%20Intensity) :!class /Script/Engine.MaterialInstanceDynamic)
  (Rendering|Material|SetScalarParameterValue _returnvalue_2 "Outline Thickness" (Variables|DashExtras|GetOutline%20Thickness) :!class /Script/Engine.MaterialInstanceDynamic)
  (Rendering|Material|SetScalarParameterValue _returnvalue_2 "Outline Distance" (Variables|DashExtras|GetOutline%20Distance) :!class /Script/Engine.MaterialInstanceDynamic)
  (bind _asmaterial_2 (Utilities|Casting|CastToMaterial (Variables|DashPostProcess/MaterialProperties|GetPost%20ToneMapping)))
  (bind _returnvalue_3 (Rendering|Material|CreateDynamicMaterialInstance _asmaterial_2 "None" "None" :!class /Script/Engine.KismetMaterialLibrary))
  ;[0.1123 0.1591 0.4948] Color Correction
  (Rendering|Material|SetScalarParameterValue _returnvalue_3 "Lens Distortion" (Variables|DashPostProcess/MaterialProperties|GetLens%20Distortion) :!class /Script/Engine.MaterialInstanceDynamic)
  (Rendering|Material|SetScalarParameterValue _returnvalue_3 "Invert Distortion" (Math|Conversions|ToFloat(Boolean) (Variables|DashPostProcess/MaterialProperties|GetInvert%20Distortion)) :!class /Script/Engine.MaterialInstanceDynamic)
  (Rendering|Material|SetScalarParameterValue _returnvalue_3 "Hue" (Variables|DashColorCorrection|GetHue) :!class /Script/Engine.MaterialInstanceDynamic)
  (Rendering|Material|SetScalarParameterValue _returnvalue_3 "Saturation" (Variables|DashColorCorrection|GetSaturation) :!class /Script/Engine.MaterialInstanceDynamic)
  (Rendering|Material|SetScalarParameterValue _returnvalue_3 "Brightness" (Variables|DashColorCorrection|GetBrightness) :!class /Script/Engine.MaterialInstanceDynamic)
  (Rendering|Material|SetScalarParameterValue _returnvalue_3 "Contrast" (Variables|DashColorCorrection|GetContrast) :!class /Script/Engine.MaterialInstanceDynamic)
  ;[0.7056 0.1112 1] Post Process Materialss
  (bind _structout (Utilities|Struct|SetmembersinWeightedBlendables (Utilities|Struct|MakeWeightedBlendables (Utilities|Array|MakeArray (Utilities|Struct|MakeWeightedBlendable _returnvalue _returnvalue_2) (Utilities|Struct|MakeWeightedBlendable _returnvalue _returnvalue_3)))))
  ;[0.08683 0.609 1] Post Process Settings
  (bind _structout_2 (Utilities|Struct|SetmembersinPostProcessSettings (Utilities|Struct|MakePostProcessSettings) "TEMP_ColorTemperature" (* (Variables|DashColorCorrection|GetTemperature) 1e+03) (Variables|DashPostProcess/MaterialProperties|GetFringe) (Variables|DashPostProcess/MaterialProperties|GetBloom) (Variables|DashPostProcess/MaterialProperties|GetDirt%20Texture) (Variables|DashPostProcess/MaterialProperties|GetDirt%20Intensity) (Variables|DashPostProcess/MaterialProperties|GetExposure) (Variables|DashPostProcess/MaterialProperties|GetDetail%20Strength) (Variables|DashPostProcess/MaterialProperties|GetVignette) (Variables|DashPostProcess/MaterialProperties|GetFilm%20Grain) (Math|Vector2D|MakeVector2D _film_grain_scale _film_grain_scale) (Variables|DashPostProcess/MaterialProperties|GetGrading%20Intensity) (Variables|DashPostProcess/MaterialProperties|GetColor%20Grading) _structout))
  (Variables|/Script/Engine.CameraComponent|SetPostProcessSettings (Variables|CameraActor|GetCameraComponent) _structout_2)
  (if (not (Variables|DashBaseProperties|GetControl%20Camera%20from%20UE%20Details%20Panel))
    ;[1 0.1719 0.1883] Camera Settings
    (bind _ascine_camera_component (Utilities|Casting|CastToCineCameraComponent (Variables|CameraActor|GetCameraComponent)))
    (Variables|Default|SetCineCameraComponent _ascine_camera_component)
    (Utilities|FlowControl|Sequence
      (:then_0
        (bind _structout_3 (Utilities|Struct|SetmembersinCameraFocusSettings (Utilities|Struct|MakeCameraFocusSettings) (* (Variables|DashBaseProperties|GetFocus%20Distance) 1e+03)))
        (Variables|/Script/CinematicCamera.CineCameraComponent|SetFocusSettings (Variables|Default|GetCineCameraComponent) _structout_3))
      (:then_1
        (bind _structout_4 (Utilities|Struct|SetmembersinCameraFilmbackSettings (Utilities|Struct|MakeCameraFilmbackSettings (Variables|DashBaseProperties|GetSensor%20Width) (Variables|DashBaseProperties|GetSensor%20Height) 0.0 0.0)))
        (Variables|/Script/CinematicCamera.CineCameraComponent|SetFilmback (Variables|Default|GetCineCameraComponent) _structout_4)
        (bind _structout_5 (Utilities|Struct|SetmembersinCameraLensSettings (Utilities|Struct|MakeCameraLensSettings 0.0 1e+03 1.2 22.0 (Variables|DashBaseProperties|GetSqueeze%20Factor))))
        (Variables|/Script/CinematicCamera.CineCameraComponent|SetLensSettings (Variables|Default|GetCineCameraComponent) _structout_5)
        (Variables|/Script/CinematicCamera.CineCameraComponent|SetCurrentFocalLength (Variables|Default|GetCineCameraComponent) (Variables|DashBaseProperties|GetFocal%20Length))
        (Variables|/Script/CinematicCamera.CineCameraComponent|SetCurrentAperture (Variables|Default|GetCineCameraComponent) (Variables|DashBaseProperties|GetAperture))))))

(event EventTick
  (params (DeltaSeconds :type Float%20%28single-precision%29))
  (CallFunction|ComputeProperties))

(fn ConstructionScript
  (CallFunction|ComputeProperties))
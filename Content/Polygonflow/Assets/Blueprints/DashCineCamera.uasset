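; Cine camera Blueprint that turns its exposed variables into post-process, lens and filmback settings.
; ComputeProperties creates dynamic instances of the pre- and post-tonemapping materials for outline, lens distortion and color correction, adding them as blendables.
; It builds fresh post-process settings for grading and film effects, then applies sensor, lens and optional focus overrides.
; Construction script is empty, and nothing in these graphs calls the event.
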(event Custom|ComputeProperties
  (bind _returnvalue (Math|Float|MakeLiteralFloat 1.0))
  (bind _film_grain_scale (Variables|DashProperties|GetFilm%20Grain%20Scale))
  ;[1 0.8918 0.2289] Outline
  (bind _asmaterial (Utilities|Casting|CastToMaterial (Variables|DashProperties|GetPre%20ToneMapping)))
  (bind _returnvalue_2 (Rendering|Material|CreateDynamicMaterialInstance _asmaterial "None" "None" :!class /Script/Engine.KismetMaterialLibrary))
  (Rendering|Material|SetScalarParameterValue _returnvalue_2 "Outline Intensity" (Variables|DashProperties|GetOutline%20Intensity) :!class /Script/Engine.MaterialInstanceDynamic)
  (Rendering|Material|SetScalarParameterValue _returnvalue_2 "Outline Thickness" (Variables|DashProperties|GetOutline%20Thickness) :!class /Script/Engine.MaterialInstanceDynamic)
  (Rendering|Material|SetScalarParameterValue _returnvalue_2 "Outline Distance" (Variables|DashProperties|GetOutline%20Distance) :!class /Script/Engine.MaterialInstanceDynamic)
  (bind _asmaterial_2 (Utilities|Casting|CastToMaterial (Variables|DashProperties|GetPost%20ToneMapping)))
  (bind _returnvalue_3 (Rendering|Material|CreateDynamicMaterialInstance _asmaterial_2 "None" "None" :!class /Script/Engine.KismetMaterialLibrary))
  ;[0.1123 0.1591 0.4948] Color Correction
  (Rendering|Material|SetScalarParameterValue _returnvalue_3 "Lens Distortion" (Variables|DashProperties|GetLens%20Distortion) :!class /Script/Engine.MaterialInstanceDynamic)
  (Rendering|Material|SetScalarParameterValue _returnvalue_3 "Invert Distortion" (Math|Conversions|ToFloat(Boolean) (Variables|DashProperties|GetInvert%20Distortion)) :!class /Script/Engine.MaterialInstanceDynamic)
  (Rendering|Material|SetScalarParameterValue _returnvalue_3 "Hue" (Variables|DashProperties|GetHue) :!class /Script/Engine.MaterialInstanceDynamic)
  (Rendering|Material|SetScalarParameterValue _returnvalue_3 "Saturation" (Variables|DashProperties|GetSaturation) :!class /Script/Engine.MaterialInstanceDynamic)
  (Rendering|Material|SetScalarParameterValue _returnvalue_3 "Brightness" (Variables|DashProperties|GetBrightness) :!class /Script/Engine.MaterialInstanceDynamic)
  (Rendering|Material|SetScalarParameterValue _returnvalue_3 "Contrast" (Variables|DashProperties|GetContrast) :!class /Script/Engine.MaterialInstanceDynamic)
  ;[0.7056 0.1112 1] Post Process Materialss
  (bind _structout (Utilities|Struct|SetmembersinWeightedBlendables (Utilities|Struct|MakeWeightedBlendables (Utilities|Array|MakeArray (Utilities|Struct|MakeWeightedBlendable _returnvalue _returnvalue_2) (Utilities|Struct|MakeWeightedBlendable _returnvalue _returnvalue_3)))))
  ;[0.08683 0.609 1] Post Process Settings
  (bind _structout_2 (Utilities|Struct|SetmembersinPostProcessSettings (Utilities|Struct|MakePostProcessSettings) "TEMP_ColorTemperature" (* (Variables|DashProperties|GetTemperature) 1e+03) (Variables|DashProperties|GetFringe) (Variables|DashProperties|GetBloom) (Variables|DashProperties|GetDirt%20Texture) (Variables|DashProperties|GetDirt%20Intensity) (Variables|DashProperties|GetExposure) (Variables|DashProperties|GetDetail%20Strength) (Variables|DashProperties|GetVignette) (Variables|DashProperties|GetFilm%20Grain) (Math|Vector2D|MakeVector2D _film_grain_scale _film_grain_scale) (Variables|DashProperties|GetGrading%20Intensity) (Variables|DashProperties|GetColor%20Grading) _structout))
  (Variables|/Script/Engine.CameraComponent|SetPostProcessSettings (Variables|CameraActor|GetCameraComponent) _structout_2)
  ;[1 0.1719 0.1883] Camera Settings
  (bind _ascine_camera_component (Utilities|Casting|CastToCineCameraComponent (Variables|CameraActor|GetCameraComponent)))
  (Variables|Default|SetCineCameraComponent _ascine_camera_component)
  (Utilities|FlowControl|Sequence
    (:then_0
      (if (Variables|DashProperties|GetOverride%20Focus%20Settings)
        (bind _structout_3 (Utilities|Struct|SetmembersinCameraFocusSettings (Utilities|Struct|MakeCameraFocusSettings) (* (Variables|DashProperties|GetFocus%20Distance) 1e+03)))
        (Variables|/Script/CinematicCamera.CineCameraComponent|SetFocusSettings (Variables|Default|GetCineCameraComponent) _structout_3)))
    (:then_1
      (bind _structout_4 (Utilities|Struct|SetmembersinCameraFilmbackSettings (Utilities|Struct|MakeCameraFilmbackSettings (Variables|DashProperties|GetSensor%20Width) (Variables|DashProperties|GetSensor%20Height) 0.0 0.0)))
      (Variables|/Script/CinematicCamera.CineCameraComponent|SetFilmback (Variables|Default|GetCineCameraComponent) _structout_4)
      (bind _structout_5 (Utilities|Struct|SetmembersinCameraLensSettings (Utilities|Struct|MakeCameraLensSettings 0.0 1e+03 1.2 22.0 (Variables|DashProperties|GetSqueeze%20Factor))))
      (Variables|/Script/CinematicCamera.CineCameraComponent|SetLensSettings (Variables|Default|GetCineCameraComponent) _structout_5)
      (Variables|/Script/CinematicCamera.CineCameraComponent|SetCurrentFocalLength (Variables|Default|GetCineCameraComponent) (Variables|DashProperties|GetFocal%20Length))
      (Variables|/Script/CinematicCamera.CineCameraComponent|SetCurrentAperture (Variables|Default|GetCineCameraComponent) (Variables|DashProperties|GetAperture)))))

(event EventBeginPlay)

(event Collision|EventActorBeginOverlap
  (params (OtherActor :type Actor%20Object%20Reference)))

(event EventTick
  (params (DeltaSeconds :type Float%20%28single-precision%29)))

(fn ConstructionScript)
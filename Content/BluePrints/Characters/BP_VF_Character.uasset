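; Player character for a third-person shooter with movement, rifle pickup, aiming and firing.
; Aiming swaps cameras and sets an ABP_Unarmed flag that gates firing.
; Firing plays effects, traces from the aim camera, pushes physics objects and calls a server fire event to damage health components.
; BP_HealthComponent changes update the health bar and, on death, disable player input and ragdoll the mesh.
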(event OnComponentBeginOverlap(CapsuleComponent)
  (params (OverlappedComponent :type Primitive%20Component%20Object%20Reference) (OtherActor :type Actor%20Object%20Reference) (OtherComp :type Primitive%20Component%20Object%20Reference) (OtherBodyIndex :type Integer) (bFromSweep :type Boolean) (SweepResult :type Hit%20Result%20Structure%20%28by%20ref%29))
  ;[0.15 0.15 0.15 0.5] IA_Weapon PickUp
  (bind _asbp_vf_wep_pickup (Utilities|Casting|CastToBP_VF_WepPickup OtherActor)))

(event Custom|Server_Fire
  (params (Start :type Vector) (End :type Vector))
  (bind _outhit (Collision|LineTraceByChannel Start End "TraceTypeQuery1" false 0 "None" true "(R=1.000000,G=0.000000,B=0.000000,A=1.000000)" "(R=0.000000,G=1.000000,B=0.000000,A=1.000000)" 0.0))
  (Utilities|IsValid (Actor|GetComponentbyClass (.HitActor (Collision|BreakHitResult _outhit)) "/Game/BluePrints/Components/BP_HealthComponent.BP_HealthComponent_C")
    (:Is%20Valid
      (Default|ReceiveDamage (Actor|GetComponentbyClass (.HitActor (Collision|BreakHitResult _outhit)) "/Game/BluePrints/Components/BP_HealthComponent.BP_HealthComponent_C") 1e+01))))

(event Custom|HandleHealthChanged
  (bind _healthbarwidget (Variables|Default|GetHealthBarWidget))
  (bind _healthcomponent (Variables|Default|GetHealthComponent))
  (Utilities|IsValid _healthbarwidget
    (:Is%20Valid
      (Default|SetFillPercent _healthbarwidget (Math|Float|SafeDivide (Variables|/Game/BluePrints/Components/BP_HealthComponent.BP_HealthComponent_C|GetHP _healthcomponent) (Variables|/Game/BluePrints/Components/BP_HealthComponent.BP_HealthComponent_C|GetMaxHP _healthcomponent))))
    (:Is%20Not%20Valid
      _))
  (if (Variables|/Game/BluePrints/Components/BP_HealthComponent.BP_HealthComponent_C|GetDied (Variables|Default|GetHealthComponent))
    (CallFunction|HandleDeath)))

(event Custom|HandleDeath
  (if (not (Variables|Default|GetbDeathHandled))
    (Variables|Default|SetbDeathHandled true)
    (bind _asplayer_controller (Utilities|Casting|CastToPlayerController (Pawn|GetController self)))
    (Utilities|IsValid _asplayer_controller
      (:Is%20Valid
        (Input|DisableInput _asplayer_controller 0)
        (Collision|SetCollisionProfileName (Variables|Character|GetMesh) "Ragdoll" true :!class /Script/Engine.PrimitiveComponent)
        (Physics|SetSimulatePhysics (Variables|Character|GetMesh) true)
        (Collision|SetCollisionEnabled (Variables|Collision|GetCapsuleComponent) "NoCollision")
        (Pawn|Components|CharacterMovement|DisableMovement (Variables|Character|GetCharacterMovement))))))

(event Input|EnhancedActionEvents|EnhancedInputActionIA_MouseLook
  (params (ActionValue :type Vector%202D%20Structure) (ElapsedSeconds :type Float%20%28double-precision%29) (TriggeredSeconds :type Float%20%28double-precision%29) (InputAction :type Input%20Action%20Object%20Reference :default "/Game/Input/Actions/IA_MouseLook.IA_MouseLook"))
  (bind (_x _y) (Math|Vector2D|BreakVector2D ActionValue))
  (bind _self self)
  ;[0.15 0.15 0.15 0.5] IA_Look / Mouse Look
  (Pawn|Input|AddControllerYawInput _self _x)
  (Pawn|Input|AddControllerPitchInput _self _y))

(event Input|EnhancedActionEvents|EnhancedInputActionIA_Jump
  (params (ActionValue :type Boolean) (ElapsedSeconds :type Float%20%28double-precision%29) (TriggeredSeconds :type Float%20%28double-precision%29) (InputAction :type Input%20Action%20Object%20Reference :default "/Game/Input/Actions/IA_Jump.IA_Jump"))
  ;[0.15 0.15 0.15 0.5] IA_Jump
  (:Started
    (Character|Jump))
  (:Completed
    (Character|StopJumping)))

(event Input|EnhancedActionEvents|EnhancedInputActionIA_PickUp
  (params (ActionValue :type Boolean) (ElapsedSeconds :type Float%20%28double-precision%29) (TriggeredSeconds :type Float%20%28double-precision%29) (InputAction :type Input%20Action%20Object%20Reference :default "/Game/Input/Actions/IA_PickUp.IA_PickUp"))
  ;[0.15 0.15 0.15 0.5] IA_Weapon PickUp
  (:Started
    (Utilities|IsValid (stale OnComponentBeginOverlap(CapsuleComponent) _asbp_vf_wep_pickup)
      (:Is%20Valid
        (if (Variables|/Game/BluePrints/Components/BP_VF_WepPickup.BP_VF_WepPickup_C|GetCanPick (stale OnComponentBeginOverlap(CapsuleComponent) _asbp_vf_wep_pickup))
          (if (not (Variables|Default|GetArmed))
            (Rendering|SetVisibility (Variables|Default|GetRifle) true false)
            (Variables|Default|SetArmed true)
            (Actor|DestroyActor (stale OnComponentBeginOverlap(CapsuleComponent) _asbp_vf_wep_pickup))))))))

(event Input|EnhancedActionEvents|EnhancedInputActionIA_Aiming
  (params (ActionValue :type Boolean) (ElapsedSeconds :type Float%20%28double-precision%29) (TriggeredSeconds :type Float%20%28double-precision%29) (InputAction :type Input%20Action%20Object%20Reference :default "/Game/Input/Actions/IA_Aiming.IA_Aiming"))
  ;[0.15 0.15 0.15 0.5] IA_Aiming
  (:Started
    (if (Variables|Default|GetArmed)
      (Components|Activation|SetActive (Variables|Default|GetAimingCamera) true false)
      (Components|Activation|SetActive (Variables|Default|GetFollowCamera) false false)
      (Variables|Default|SetbUseControllerRotationYaw true)
      (bind _asabp_unarmed (Utilities|Casting|CastToABP_Unarmed (Components|SkeletalMesh|GetAnimInstance (Variables|Character|GetMesh))))
      (Variables|/Game/Characters/Mannequins/Anims/Unarmed/ABP_Unarmed.ABP_Unarmed_C|SetIsAiming _asabp_unarmed true)))
  (:Canceled
    (if (Variables|Default|GetArmed) :!label _label
      (Components|Activation|SetActive (Variables|Default|GetAimingCamera) false false)
      (Components|Activation|SetActive (Variables|Default|GetFollowCamera) true false)
      (Variables|Default|SetbUseControllerRotationYaw true)
      (bind _asabp_unarmed_2 (Utilities|Casting|CastToABP_Unarmed (Components|SkeletalMesh|GetAnimInstance (Variables|Character|GetMesh))))
      (Variables|/Game/Characters/Mannequins/Anims/Unarmed/ABP_Unarmed.ABP_Unarmed_C|SetIsAiming _asabp_unarmed_2 true)))
  (:Completed
    (goto _label)))

(event Input|EnhancedActionEvents|EnhancedInputActionIA_Fire
  (params (ActionValue :type Boolean) (ElapsedSeconds :type Float%20%28double-precision%29) (TriggeredSeconds :type Float%20%28double-precision%29) (InputAction :type Input%20Action%20Object%20Reference :default "/Game/Input/Actions/IA_Fire.IA_Fire"))
  (bind _firepoint (Variables|Default|GetFirePoint))
  (bind _aimingcamera (Variables|Default|GetAimingCamera))
  (bind _gunrange (Variables|Default|GetGunRange))
  (bind _returnvalue (Math|Vector|GetForwardVector _aimingcamera))
  (bind _returnvalue_2 (Transformation|GetWorldLocation _firepoint))
  (bind _returnvalue_3 (Transformation|GetWorldLocation _aimingcamera))
  (bind _returnvalue_4 (* _returnvalue _gunrange))
  (bind _returnvalue_5 (+ _returnvalue_3 _returnvalue_4))
  ;[0.15 0.15 0.15 0.5] IA_Fire
  (:Started
    (if (Variables|Default|GetArmed)
      (bind _asabp_unarmed (Utilities|Casting|CastToABP_Unarmed (Components|SkeletalMesh|GetAnimInstance (Variables|Character|GetMesh))))
      (if (Variables|/Game/Characters/Mannequins/Anims/Unarmed/ABP_Unarmed.ABP_Unarmed_C|GetIsAiming _asabp_unarmed)
        (Animation|PlayAnimMontage "/Game/Anims/ANIM_VF_Fire_Rifle_Hip_Montage.ANIM_VF_Fire_Rifle_Hip_Montage" 1.0 "None")
        (Audio|PlaySoundatLocation "/Game/Weapons/GrenadeLauncher/Audio/FirstPersonTemplateWeaponFire02.FirstPersonTemplateWeaponFire02" _returnvalue_2 "0, 0, 0" 1.0 1.0 0.0 0 0 0 0)
        (Niagara|SpawnSystematLocation "/Game/MuzzleFlash/MuzzleFlash/Niagara/NS_MuzzleFlash.NS_MuzzleFlash" _returnvalue_2 (Transformation|GetWorldRotation _firepoint))
        (bind _outhit (Collision|LineTraceByChannel _returnvalue_3 _returnvalue_5 "TraceTypeQuery1" false 0 "ForDuration" true "(R=1.000000,G=0.000000,B=0.000000,A=1.000000)" "(R=0.000000,G=1.000000,B=0.000000,A=1.000000)" 2.0))
        (Rendering|Decal|SpawnDecalatLocation (.OutItem (Utilities|Array|Random (Variables|Default|GetBulletsImpactMap))) (Math|Conversions|ToVector(Float) (Math|Random|RandomFloatinRange 0.0 0.0)) (.ImpactPoint (Collision|BreakHitResult _outhit)) (Math|Rotator|FindLookatRotation (.TraceStart (Collision|BreakHitResult _outhit)) (.TraceEnd (Collision|BreakHitResult _outhit))) 2e+01)
        (Utilities|IsValid (.HitComponent (Collision|BreakHitResult _outhit))
          (:Is%20Valid
            (Utilities|FlowControl|Sequence
              (:then_0
                (if (Physics|IsSimulatingPhysics (.HitComponent (Collision|BreakHitResult _outhit)) "None")
                  (Physics|AddImpulseatLocation (.HitComponent (Collision|BreakHitResult _outhit)) (* (Math|Vector|GetUnitDirection(Vector) (.TraceStart (Collision|BreakHitResult _outhit)) (.TraceEnd (Collision|BreakHitResult _outhit))) (Variables|Default|GetFireRateMultiplier)) (.ImpactPoint (Collision|BreakHitResult _outhit)) "None")))
              (:then_1
                (CallFunction|ServerFire _returnvalue_3 _returnvalue_5)))))))))

(event Input|EnhancedActionEvents|EnhancedInputActionIA_Move
  (params (ActionValue :type Vector%202D%20Structure) (ElapsedSeconds :type Float%20%28double-precision%29) (TriggeredSeconds :type Float%20%28double-precision%29) (InputAction :type Input%20Action%20Object%20Reference :default "/Game/Input/Actions/IA_Move.IA_Move"))
  (bind (_x _y) (Math|Vector2D|BreakVector2D ActionValue))
  (bind _self self)
  (bind _returnvalue (Pawn|GetController _self))
  (bind _returnvalue_2 (Pawn|GetControlRotation _returnvalue :!class /Script/Engine.Controller))
  (bind _yaw (Math|Rotator|BreakRotator _returnvalue_2))
  (bind _returnvalue_3 (Math|Rotator|MakeRotator 0.0 0.0 _yaw))
  ;[0.15 0.15 0.15 0.5] IA_Move
  (Utilities|IsValid _returnvalue
    (:Is%20Valid
      (Pawn|Input|AddMovementInput self (Math|Vector|GetForwardVector _returnvalue_3) _y false)
      (Pawn|Input|AddMovementInput self (Math|Vector|GetRightVector _returnvalue_3) _x false))))

(event Input|EnhancedActionEvents|EnhancedInputActionIA_Look
  (params (ActionValue :type Vector%202D%20Structure) (ElapsedSeconds :type Float%20%28double-precision%29) (TriggeredSeconds :type Float%20%28double-precision%29) (InputAction :type Input%20Action%20Object%20Reference :default "/Game/Input/Actions/IA_Look.IA_Look"))
  (bind (_x _y) (Math|Vector2D|BreakVector2D ActionValue))
  (bind _self self)
  ;[0.15 0.15 0.15 0.5] IA_Look / Mouse Look
  (Pawn|Input|AddControllerYawInput _self _x)
  (Pawn|Input|AddControllerPitchInput _self _y))

(event Game|Damage|EventAnyDamage
  (params (Damage :type Float%20%28single-precision%29) (DamageType :type Damage%20Type%20Object%20Reference) (InstigatedBy :type Controller%20Object%20Reference) (DamageCauser :type Actor%20Object%20Reference))
  (Default|ReceiveDamage (Variables|Default|GetHealthComponent) Damage))

(event EventBeginPlay
  (EventDispatchers|BindEventtoOnHealthChanged (Variables|Default|GetHealthComponent) (EventDispatchers|CreateEvent :!event Custom|HandleHealthChanged))
  (if (Pawn|IsLocallyControlled)
    (bind _returnvalue (UserInterface|CreateWidget "/Game/Synty/UIMilitaryCombatHUD/Widgets/Reticles_Crosshairs/HUD_MilitaryCombat_Reticle_Crosshair_01.HUD_MilitaryCombat_Reticle_Crosshair_01_C"))
    (Variables|Default|SetCrosshairWidget _returnvalue)
    (UserInterface|Viewport|AddtoViewport (Variables|Default|GetCrosshairWidget) 0)
    (bind _returnvalue_2 (UserInterface|CreateWidget "/Game/Synty/UIMilitaryCombatHUD/Widgets/Player_Health_Equipment/HUD_MilitaryCombat_HealthBar_03.HUD_MilitaryCombat_HealthBar_03_C"))
    (Variables|Default|SetHealthBarWidget _returnvalue_2)
    (UserInterface|Viewport|AddtoViewport _returnvalue_2 0)))

(fn ConstructionScript)

(fn Aim
  (params (X%20Axis :type Float%20%28single-precision%29) (Y%20Axis :type Float%20%28double-precision%29)))

(fn Move
  (params (X%20Axis :type Float%20%28double-precision%29) (Y%20Axis :type Float%20%28double-precision%29)))

(fn OnRepHealth)
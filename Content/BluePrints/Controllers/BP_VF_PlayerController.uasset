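; BP_VF_PlayerController is a player controller that sets up input and a Steam session component when play begins.
; For a local controller only, it adds the default and mouse-look Enhanced Input mapping contexts to player index 0's subsystem at equal priority.
; It then passes itself to SteamSeshComp and initializes that component, leaving any session logic to it.
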(event EventBeginPlay
  (bind _returnvalue (Game|GetPlayerController 0))
  (bind _returnvalue_2 (PlayerController|LocalPlayerSubsystems|GetEnhancedInputLocalPlayerSubsystem _returnvalue))
  (if (Pawn|IsLocalPlayerController)
    (Utilities|FlowControl|Sequence
      (:then_0
        (Input|AddMappingContext _returnvalue_2 "/Game/Input/IMC_Default.IMC_Default" 0 "(bIgnoreAllPressedKeysUntilRelease=True,bForceImmediately=False,bNotifyUserSettings=False)")
        (Input|AddMappingContext _returnvalue_2 "/Game/Input/IMC_MouseLook.IMC_MouseLook" 0 "(bIgnoreAllPressedKeysUntilRelease=True,bForceImmediately=False,bNotifyUserSettings=False)"))
      (:then_1
        (Variables|/Game/Steam/SteamSeshComp.SteamSeshComp_C|SetPlayer%20Controller (Variables|Default|GetSteamSeshComp) self)
        (Default|InitializeController (Variables|Default|GetSteamSeshComp))))))

(fn ConstructionScript)
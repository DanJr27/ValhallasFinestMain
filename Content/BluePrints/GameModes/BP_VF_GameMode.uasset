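; Game mode for round-based Alpha versus Bravo elimination matches, automatically restarting rounds after a delay.
; StartRound resets game state and respawns players, while ChoosePlayerStart assigns unteamed players to the smaller team and picks a random team-tagged start.
; A looping one-second RoundTick ends the round through EndRound when a team is eliminated or time expires.
; DetermineTimeoutWinner counts team "None" for both sides, so timeouts always yield a Draw.
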(event Custom|StartRound
  (bind _self self)
  (bind _asbp_vf_game_state (Utilities|Casting|CastToBP_VF_GameState (Game|GetGameState)))
  (Variables|/Game/BluePrints/States/BP_VF_GameState.BP_VF_GameState_C|SetRoundState _asbp_vf_game_state "InProgress")
  (Variables|/Game/BluePrints/States/BP_VF_GameState.BP_VF_GameState_C|SetWinningTeam _asbp_vf_game_state "None")
  (Variables|/Game/BluePrints/States/BP_VF_GameState.BP_VF_GameState_C|SetMatchTimeRemaining _asbp_vf_game_state (Variables|Default|GetRoundDurationSeconds))
  (for _array_element (Variables|/Script/Engine.GameStateBase|GetPlayerArray (Game|GetGameState))
    (bind _asbp_vf_player_state (Utilities|Casting|CastToBP_VF_PlayerState _array_element))
    (Variables|/Game/BluePrints/States/BP_VF_PlayerState.BP_VF_PlayerState_C|SetbIsEliminated _asbp_vf_player_state false)
    (Utilities|IsValid (Game|GetPlayerController _asbp_vf_player_state)
      (:Is%20Valid
        (Utilities|IsValid (PlayerState|GetPawn _asbp_vf_player_state)
          (:Is%20Valid
            (Actor|DestroyActor (PlayerState|GetPawn _asbp_vf_player_state))
            (Class|GameModeBase|RestartPlayer _self (Game|GetPlayerController _asbp_vf_player_state)))
          (:Is%20Not%20Valid
            (Class|GameModeBase|RestartPlayer _self (Game|GetPlayerController _asbp_vf_player_state)))))))
  (Utilities|Time|SetTimerbyFunctionName _self "RoundTick" 1.0 true))

(event Custom|RoundTick
  (bind _self self)
  (bind _asbp_vf_game_state (Utilities|Casting|CastToBP_VF_GameState (Game|GetGameState)))
  (Variables|/Game/BluePrints/States/BP_VF_GameState.BP_VF_GameState_C|SetMatchTimeRemaining _asbp_vf_game_state (- (Variables|/Game/BluePrints/States/BP_VF_GameState.BP_VF_GameState_C|GetMatchTimeRemaining _asbp_vf_game_state) (Math|Float|MakeLiteralFloat 1.0)))
  (bind _returnvalue (CallFunction|CountAlivebyTeam _self "Alpha"))
  (bind _returnvalue_2 (CallFunction|CountAlivebyTeam _self "Bravo"))
  (if (and (== _returnvalue (Class|KismetSystemLibrary|MakeLiteralInteger)) (== _returnvalue_2 (Class|KismetSystemLibrary|MakeLiteralInteger)))
    (CallFunction|EndRound _self "Draw")
    (elif (== _returnvalue (Class|KismetSystemLibrary|MakeLiteralInteger))
      (CallFunction|EndRound _self "Bravo")
      (elif (== _returnvalue_2 (Class|KismetSystemLibrary|MakeLiteralInteger))
        (CallFunction|EndRound _self "Alpha")
        (elif (<= (- (Variables|/Game/BluePrints/States/BP_VF_GameState.BP_VF_GameState_C|GetMatchTimeRemaining _asbp_vf_game_state) (Math|Float|MakeLiteralFloat 1.0)) (Math|Float|MakeLiteralFloat 0.0))
          (bind _returnvalue_3 (CallFunction|DetermineTimeoutWinner _self))
          (CallFunction|EndRound _self _returnvalue_3))))))

(event EventBeginPlay
  (Development|PrintString "BP_VF_GameMode Loaded")
  (CallFunction|StartRound))

(event EventTick
  (params (DeltaSeconds :type Float%20%28single-precision%29)))

(fn ConstructionScript)

(fn ChoosePlayerStart
  (params (Player :type Controller%20Object%20Reference))
  (bind _asbp_vf_player_state (Utilities|Casting|CastToBP_VF_PlayerState (Variables|/Script/Engine.Controller|GetPlayerState Player))
    (:then
      (if (== (Variables|/Game/BluePrints/States/BP_VF_PlayerState.BP_VF_PlayerState_C|GetTeamTag _asbp_vf_player_state) (Utilities|String|MakeLiteralString "None"))
        (Variables|Default|SetTempAlphaCount 0)
        (Variables|Default|SetTempBravoCount 0)
        (for _array_element (Variables|/Script/Engine.GameStateBase|GetPlayerArray (Game|GetGameState))
          (bind _asbp_vf_player_state_2 (Utilities|Casting|CastToBP_VF_PlayerState _array_element))
          (if (== (Variables|/Game/BluePrints/States/BP_VF_PlayerState.BP_VF_PlayerState_C|GetTeamTag _asbp_vf_player_state_2) (Utilities|String|MakeLiteralString "Alpha"))
            (Variables|Default|SetTempAlphaCount (+ (Variables|Default|GetTempAlphaCount) (Class|KismetSystemLibrary|MakeLiteralInteger 1)))
            (elif (== (Variables|/Game/BluePrints/States/BP_VF_PlayerState.BP_VF_PlayerState_C|GetTeamTag _asbp_vf_player_state_2) (Utilities|String|MakeLiteralString "Bravo"))
              (Variables|Default|SetTempBravoCount (+ (Variables|Default|GetTempBravoCount) (Class|KismetSystemLibrary|MakeLiteralInteger 1))))))
        (Variables|Default|SetChosenTeam (Utilities|String|StringToName (select (<= (Variables|Default|GetTempAlphaCount) (Variables|Default|GetTempBravoCount)) (Utilities|String|MakeLiteralString "Alpha") (Utilities|String|MakeLiteralString "Bravo"))))
        (Variables|/Game/BluePrints/States/BP_VF_PlayerState.BP_VF_PlayerState_C|SetTeamTag _asbp_vf_player_state (Variables|Default|GetChosenTeam))
        (else
          (Variables|Default|SetChosenTeam (Variables|/Game/BluePrints/States/BP_VF_PlayerState.BP_VF_PlayerState_C|GetTeamTag _asbp_vf_player_state))))
      (bind _outactors (Actor|GetAllActorswithTag (Variables|Default|GetChosenTeam)))
      (if (> (Utilities|Array|Length _outactors) (Class|KismetSystemLibrary|MakeLiteralInteger))
        (return (Utilities|Array|Get(acopy) _outactors (Math|Random|RandomIntegerinRange 0 (- (Utilities|Array|Length _outactors) (Class|KismetSystemLibrary|MakeLiteralInteger 1)))))
        (else
          (return 0))))
    (:CastFailed
      (return 0))))

(fn EndRound
  (params (Winner :type Name))
  (bind _self self)
  (Utilities|Time|ClearTimerbyFunctionName _self "RoundTick")
  (bind _asbp_vf_game_state (Utilities|Casting|CastToBP_VF_GameState (Game|GetGameState)))
  (Variables|/Game/BluePrints/States/BP_VF_GameState.BP_VF_GameState_C|SetRoundState _asbp_vf_game_state "RoundEnd")
  (Variables|/Game/BluePrints/States/BP_VF_GameState.BP_VF_GameState_C|SetWinningTeam _asbp_vf_game_state Winner)
  (Utilities|Time|SetTimerbyFunctionName _self "StartRound" 8.0))

(fn CountAlivebyTeam
  (params (TeamName :type Name))
  (Variables|Default|SetTempCount 0)
  (for _array_element (Variables|/Script/Engine.GameStateBase|GetPlayerArray (Game|GetGameState))
    (bind _asbp_vf_player_state (Utilities|Casting|CastToBP_VF_PlayerState _array_element))
    (if (and (== (Variables|/Game/BluePrints/States/BP_VF_PlayerState.BP_VF_PlayerState_C|GetTeamTag _asbp_vf_player_state) TeamName) (not (Variables|/Game/BluePrints/States/BP_VF_PlayerState.BP_VF_PlayerState_C|GetbIsEliminated _asbp_vf_player_state)))
      (Variables|Default|SetTempCount (+ (Variables|Default|GetTempCount) (Class|KismetSystemLibrary|MakeLiteralInteger 1)))))
  (return (Variables|Default|GetTempCount)))

(fn DetermineTimeoutWinner
  (bind _returnvalue (CallFunction|CountAlivebyTeam "None"))
  (bind _returnvalue_2 (CallFunction|CountAlivebyTeam "None"))
  (return (Utilities|String|StringToName (select (== _returnvalue _returnvalue_2) (Utilities|String|MakeLiteralString "Draw") (select (> _returnvalue _returnvalue_2) (Utilities|String|MakeLiteralString "Alpha") (Utilities|String|MakeLiteralString "Bravo"))))))

(fn CountTotalbyTeam
  (params (TeamName :type Name))
  (Variables|Default|SetTempCount 0)
  (for _array_element (Variables|/Script/Engine.GameStateBase|GetPlayerArray (Game|GetGameState))
    (bind _asbp_vf_player_state (Utilities|Casting|CastToBP_VF_PlayerState _array_element))
    (if (== (Variables|/Game/BluePrints/States/BP_VF_PlayerState.BP_VF_PlayerState_C|GetTeamTag _asbp_vf_player_state) TeamName)
      (Variables|Default|SetTempCount (+ (Variables|Default|GetTempCount) (Class|KismetSystemLibrary|MakeLiteralInteger 1)))))
  (return (Variables|Default|GetTempCount)))
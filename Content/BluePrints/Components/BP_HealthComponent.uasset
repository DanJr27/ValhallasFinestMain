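; Health component that tracks HP, health percentage and death state for its owning actor, with rep-notify replication.
; ReceiveDamage subtracts clamped damage and ResetHealth restores full health, both calling OnHealthChanged after updating state.
; OnRep handlers repeat the health-change and death notifications when HP or Died replicates.
; NotifyDied casts the owner to BP_VF_Character and calls HandleDeath when Died is set.
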(event EventBeginPlay)

(event EventTick
  (params (DeltaSeconds :type Float%20%28single-precision%29)))

(fn ReceiveDamage
  (params (Amount :type Float%20%28double-precision%29))
  (bind _output_get (Variables|Default|SetHP (Math|Float|Clamp(Float) (- (Variables|Default|GetHP) Amount) 0.0 (Variables|Default|GetMaxHP))))
  (Variables|Default|SetHealthPercentage (/ _output_get (Variables|Default|GetMaxHP)))
  (Variables|Default|SetDied (<= _output_get (Class|KismetSystemLibrary|MakeLiteralInteger)))
  (Default|CallOnHealthChanged)
  (CallFunction|NotifyDied))

(fn ResetHealth
  (Variables|Default|SetHP (Variables|Default|GetMaxHP))
  (Variables|Default|SetHealthPercentage 1.0)
  (Variables|Default|SetDied false)
  (Default|CallOnHealthChanged))

(fn OnRepHP
  (Default|CallOnHealthChanged))

(fn OnRepDied
  (CallFunction|NotifyDied))

(fn NotifyDied
  (if (Variables|Default|GetDied)
    (bind _asbp_vf_character (Utilities|Casting|CastToBP_VF_Character (Components|GetOwner)))
    (Default|HandleDeath _asbp_vf_character)))
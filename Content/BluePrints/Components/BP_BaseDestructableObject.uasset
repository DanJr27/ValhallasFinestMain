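; BP_BaseDestructableObject is a target dummy actor with a health bar that restores its health after dying.
; On BeginPlay it binds to the health component's OnHealthChanged event and resets health.
; Each change pushes the health percentage into the EnemyHealthBar progress bar in its widget component.
; If the component reports death, health resets after a short delay; nothing in the graph destroys the actor.
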(event Custom|OnHealthChanged_Event
  (bind _bp_healthcomponent (Variables|Default|GetBP_HealthComponent))
  ;[0.15 0.15 0.15 0.5] Target Dummy
  (bind _asenemy_health_bar (Utilities|Casting|CastToEnemyHealthBar (UserInterface|GetWidget (Variables|Default|GetWidget))))
  (Progress|SetPercent (Variables|/Game/UI/EnemyHealthBar.EnemyHealthBar_C|GetHealthProgresBar _asenemy_health_bar) (Variables|/Game/BluePrints/Components/BP_HealthComponent.BP_HealthComponent_C|GetHealthPercentage _bp_healthcomponent))
  (if (Variables|/Game/BluePrints/Components/BP_HealthComponent.BP_HealthComponent_C|GetDied _bp_healthcomponent)
    (Utilities|FlowControl|Delay 1.5)
    (Default|ResetHealth _bp_healthcomponent)))

(event Collision|EventActorBeginOverlap
  (params (OtherActor :type Actor%20Object%20Reference)))

(event EventTick
  (params (DeltaSeconds :type Float%20%28single-precision%29)))

(event EventBeginPlay
  (bind _bp_healthcomponent (Variables|Default|GetBP_HealthComponent))
  ;[0.15 0.15 0.15 0.5] Target Dummy
  (EventDispatchers|AssignOnHealthChanged _bp_healthcomponent (delegate Custom|OnHealthChanged_Event))
  (Default|ResetHealth _bp_healthcomponent))

(fn ConstructionScript)